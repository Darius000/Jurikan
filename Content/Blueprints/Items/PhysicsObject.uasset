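; PhysicsObject is an item actor that rides the ocean surface by following the wave height.
; On BeginPlay it teleports vertically to the OceanBp actor's height.
; Each Tick it feeds OceanBp's wave parameters, its location and game time into OceanManager's GetWaveHeightValue, then sets its Z directly rather than simulating buoyancy.
; SetForce, despite its name, overwrites the static mesh's physics linear velocity.
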(event EventBeginPlay
  (bind _returnvalue (Transformation|GetActorLocation))
  (bind (_x _y) (Math|Vector|BreakVector _returnvalue))
  (Transformation|SetActorLocation (Math|Vector|MakeVector _x _y (.Z (Math|Vector|BreakVector (Transformation|GetActorLocation (Variables|Default|GetOceanBp))))) false true))

(event Collision|EventActorBeginOverlap
  (params (OtherActor :type Actor%20Object%20Reference)))

(event EventTick
  (params (DeltaSeconds :type Float%20%28single-precision%29))
  (bind _returnvalue (Transformation|GetActorLocation))
  (bind (_x _y) (Math|Vector|BreakVector _returnvalue))
  (bind (_amp1 _amp2 _wave1 _wav2 _direction) (Default|GetOceanWaves (Variables|Default|GetOceanBp)))
  (bind _returnvalue_2 (Class|OceanManager|GetWaveHeightValue (Variables|Default|GetOceanManager) _wave1 _wav2 _amp1 _amp2 (Transformation|GetActorLocation) (Math|Vector2D|MakeVector2D (.X (Math|Vector|BreakVector _direction)) (.Y (Math|Vector|BreakVector _direction))) (Utilities|Time|GetGameTimeinSeconds)))
  (Transformation|SetActorLocation (Math|Vector|MakeVector _x _y (+ (.z (Transformation|GetActorLocation (Variables|Default|GetOceanBp))) (.Z (Math|Vector|BreakVector _returnvalue_2)))) false false))

(fn ConstructionScript)

(fn SetForce
  (params (New%20Force :type Vector))
  (Class|PrimitiveComponent|SetAllPhysicsLinearVelocity (Variables|Default|GetStaticMesh) New%20Force false))