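; FishManager is a trigger-volume spawner that populates an area with random actors, presumably fish, while a Boat is inside.
; On Boat entry, it spawns random ActorsToSpawn classes at random reachable navigation points around itself and records them in ActorsSpawned.
; On Boat exit, it loops over that array to destroy them, but empties it inside the loop.
; The construction script sizes the box from SpawnLocation.
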(event OnComponentBeginOverlap(Box)
  (params (OverlappedComponent :type Primitive%20Component%20Object%20Reference) (OtherActor :type Actor%20Object%20Reference) (OtherComp :type Primitive%20Component%20Object%20Reference) (OtherBodyIndex :type Integer) (bFromSweep :type Boolean) (SweepResult :type Hit%20Result%20Structure%20%28by%20ref%29))
  (bind _returnvalue (Transformation|GetActorLocation))
  (bind _returnvalue_2 (AI|Navigation|GetRandomReachablePointinRadius _returnvalue 2e+03))
  (Utilities|Casting|CastToBoat OtherActor)
  (for _index (range 0 (Variables|Default|GetSpawnAmount))
    (bind _returnvalue_3 (Game|SpawnActorfromClass (Utilities|Array|Get(acopy) (Variables|Default|GetActorsToSpawn) (Math|Random|RandomIntegerinRange 0 (- (Utilities|Array|Length (Variables|Default|GetActorsToSpawn)) 1))) (Math|Transform|MakeTransform (Math|Vector|MakeVector (.x _returnvalue_2) (.y _returnvalue_2) (.z _returnvalue_2)) "0, 0, 0" "1,1,1") "AdjustIfPossibleButAlwaysSpawn" 0 0))
    (Utilities|Array|Add (Variables|Default|GetActorsSpawned) _returnvalue_3)))

(event OnComponentEndOverlap(Box)
  (params (OverlappedComponent :type Primitive%20Component%20Object%20Reference) (OtherActor :type Actor%20Object%20Reference) (OtherComp :type Primitive%20Component%20Object%20Reference) (OtherBodyIndex :type Integer))
  (Utilities|Casting|CastToBoat OtherActor)
  (for _array_element (Variables|Default|GetActorsSpawned)
    (if (!= _array_element 0)
      (Actor|DestroyActor _array_element)
      (Utilities|Array|Resize (Variables|Default|GetActorsSpawned) 0))))

(event EventBeginPlay)

(event Collision|EventActorBeginOverlap
  (params (OtherActor :type Actor%20Object%20Reference)))

(event EventTick
  (params (DeltaSeconds :type Float%20%28single-precision%29)))

(fn ConstructionScript
  (Components|Box|SetBoxExtent (Variables|Default|GetBox) (Variables|Default|GetSpawnLocation) true))