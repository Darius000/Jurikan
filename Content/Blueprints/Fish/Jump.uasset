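; Behavior tree task that makes an AI-controlled fish play its jump animation.
; When the IsJumping blackboard flag is set, it casts the Fish mesh's anim instance to the medium fish Anim Blueprint, falling back to the small fish one, and calls JumpEvent on it.
; It then finishes successfully, also when the flag is unset, but never calls FinishExecute if both casts fail.
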(event EventReceiveExecuteAI
  (params (OwnerController :type AI%20Controller%20Object%20Reference) (ControlledPawn :type Pawn%20Object%20Reference))
  (bind _asfish (Utilities|Casting|CastToFish ControlledPawn))
  (bind _mesh (Variables|/Script/Engine.Character|GetMesh _asfish))
  (bind _returnvalue (Components|SkeletalMesh|GetAnimInstance _mesh))
  (if (Class|BTFunctionLibrary|GetBlackboardValueasBool (Variables|Default|GetIsJumping))
    (bind _asmedium_fish_anim (Utilities|Casting|CastToMedium_Fish_Anim _returnvalue)
      (:then
        (Default|JumpEvent _asmedium_fish_anim))
      (:CastFailed
        (bind _assmall_fisj_anim_bp (Utilities|Casting|CastToSmall_Fisj_Anim_Bp _returnvalue))
        (Default|JumpEvent _assmall_fisj_anim_bp))))
  (AI|BehaviorTree|FinishExecute true))