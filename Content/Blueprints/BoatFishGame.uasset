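; BoatFishGame manages the HUD and win check for what its name suggests is a boat fishing game.
; On BeginPlay it creates the HUD widget and adds it to the viewport.
; CheckPoints reads CurrentPoints from the HUD, sets Win only when the score exceeds a fixed threshold, and passes the result to the HUD's WinLose.
; The score is read from the widget, and nothing in this Blueprint calls CheckPoints.
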(event Custom|CheckPoints
  (bind _hud (Variables|Default|GetHUD))
  (if (> (Variables|/Game/Blueprints/HUD.HUD_C|GetCurrentPoints _hud) 50)
    (Variables|Default|SetWin? true)
    (else
      (Variables|Default|SetWin? false)))
  (Default|WinLose _hud (Variables|Default|GetWin?)))

(event EventBeginPlay
  (bind _returnvalue (UserInterface|CreateWidget "/Game/Blueprints/HUD.HUD_C"))
  (bind _output_get (Variables|Default|SetHUD _returnvalue))
  (UserInterface|Viewport|AddtoViewport _output_get 0))

(event EventTick
  (params (DeltaSeconds :type Float%20%28single-precision%29)))

(fn ConstructionScript)