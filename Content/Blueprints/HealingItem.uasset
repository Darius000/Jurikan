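; HealingItem is a pickup actor that heals a Boat when one overlaps it.
; On overlap it passes its heal amount to the boat's HealBoat and plays a pickup sound at its own location.
; It then removes itself from the Actors collection under the ocean Blueprint's Wind before destroying itself.
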(event EventBeginPlay)

(event EventTick
  (params (DeltaSeconds :type Float%20%28single-precision%29)))

(event Collision|EventActorBeginOverlap
  (params (OtherActor :type Actor%20Object%20Reference))
  (bind _asboat (Utilities|Casting|CastToBoat OtherActor))
  (Default|HealBoat _asboat (Variables|Default|GetHealAmount))
  (Audio|PlaySoundatLocation "/Game/Sound/item_pickup_sound.item_pickup_sound" (Transformation|GetActorLocation))
  (Utilities|Array|RemoveItem (Variables|/Game/Blueprints/Wind_Bp.Wind_Bp_C|GetActors (Variables|/Game/Blueprints/Ocean_Bp.Ocean_Bp_C|GetWind (Variables|Default|GetOceanBp))) self)
  (Actor|DestroyActor))

(fn ConstructionScript)