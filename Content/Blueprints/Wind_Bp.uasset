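; Wind controller Blueprint that lets player input steer a global wind and broadcasts it to the actors in the level.
; BeginPlay caches every Actor in the level, and each Tick sends the current speed and direction to all of them through WindMessage, without filtering.
; Axis inputs incrementally adjust the clamped speed and X/Y components, which form an unnormalized horizontal direction vector.
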(event EventBeginPlay
  ;[1 1 1] Get All Actors to be effected by Wind
  (bind _outactors (Actor|GetAllActorsOfClass "/Script/Engine.Actor"))
  (for _array_element _outactors
    (Utilities|Array|Add (Variables|Default|GetActors) _array_element)))

(event EventTick
  (params (DeltaSeconds :type Float%20%28single-precision%29))
  ;[1 1 1] Change Wind Speed
  (CallFunction|ChangeWind (Variables|Wind|GetSpeed) (Variables|Wind|GetDirection)))

(event Input|AxisEvents|InputAxisWindDirectionX
  (params (AxisValue :type Float%20%28single-precision%29))
  ;[1 1 1] Change Wind Direction
  (Variables|Default|SetWindXDirection (Math|Float|Clamp(Float) (+ (Variables|Default|GetWindXDirection) (* AxisValue (Variables|Default|GetRate))) -1.0))
  (Variables|Wind|SetDirection (Math|Vector|MakeVector (Variables|Default|GetWindXDirection) (Variables|Default|GetWindYDirection) 0.0)))

(event Input|AxisEvents|InputAxisWindDirectionY
  (params (AxisValue :type Float%20%28single-precision%29))
  ;[1 1 1] Change Wind Direction
  (Variables|Default|SetWindYDirection (Math|Float|Clamp(Float) (+ (Variables|Default|GetWindYDirection) (* AxisValue (Variables|Default|GetRate))) -1.0))
  (Variables|Wind|SetDirection (Math|Vector|MakeVector (Variables|Default|GetWindXDirection) (Variables|Default|GetWindYDirection) 0.0)))

(event Input|AxisEvents|InputAxisChangeSpeed
  (params (AxisValue :type Float%20%28single-precision%29))
  ;[1 1 1] Change Wind Speed
  (Variables|Wind|SetSpeed (Math|Float|Clamp(Float) (+ (Variables|Wind|GetSpeed) (* AxisValue (Variables|Default|GetSpeedRate))) 0.0 157.0)))

(fn ConstructionScript)

(fn ChangeWind
  (params (Speed :type Float%20%28single-precision%29) (Direction :type Vector))
  (for _array_element (Variables|Default|GetActors)
    (Class|Interactions|Wind(Message) _array_element Direction Speed)))