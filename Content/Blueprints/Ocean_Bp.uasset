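; Ocean surface actor that drives a wave material from a Wind reference and tracks wave height at its own location.
; Construction applies scale and material, with a RefreshWaves toggle that rebuilds the dynamic instance and seeds wind values or defaults.
; Each Tick pushes wind direction and speed to the material, reads its wave parameters back, and has OceanManager compute WaveOffset from them and game time.
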(event EventBeginPlay)

(event Collision|EventActorBeginOverlap
  (params (OtherActor :type Actor%20Object%20Reference)))

(event EventTick
  (params (DeltaSeconds :type Float%20%28single-precision%29))
  (bind _wind (Variables|Default|GetWind))
  (Variables|Default|SetDeltaTime DeltaSeconds)
  (CallFunction|SetOceanWaves (Variables|/Game/Blueprints/Wind_Bp.Wind_Bp_C|GetDirection _wind) (Variables|/Game/Blueprints/Wind_Bp.Wind_Bp_C|GetSpeed _wind))
  (bind (_amp1 _amp2 _wave1 _wav2 _direction) (CallFunction|GetOceanWaves))
  (bind _returnvalue (Class|OceanManager|GetWaveHeightValue (Variables|Default|GetOceanManager) _amp1 _amp2 _wave1 _wav2 (Transformation|GetActorLocation) (Math|Vector2D|MakeVector2D (.X (Math|Vector|BreakVector _direction)) (.Y (Math|Vector|BreakVector _direction))) (Utilities|Time|GetGameTimeinSeconds)))
  (Variables|Default|SetWaveOffset _returnvalue))

(fn ConstructionScript
  (bind _scale (Variables|Default|GetScale))
  (bind _wind (Variables|Default|GetWind))
  (bind (_x _y) (Math|Vector2D|BreakVector2D _scale))
  (Transformation|SetActorScale3D (Math|Vector|MakeVector _x _y 1.0))
  (Rendering|Material|SetMaterial (Variables|Default|GetOcean) 0 (Variables|Default|GetOceanMaterial))
  (if (Variables|Default|GetRefreshWaves)
    (Variables|Default|SetRefreshWaves false)
    (Utilities|FlowControl|Sequence
      (:then_0
        (bind _returnvalue (Rendering|Material|CreateDynamicMaterialInstance (Variables|Default|GetOcean) 0 "/Game/Material/Ocean_Inst.Ocean_Inst" :!class /Script/Engine.PrimitiveComponent))
        (Variables|Default|SetDynamicMaterial _returnvalue))
      (:then_1
        (if (!= _wind 0)
          (CallFunction|SetOceanWaves (Variables|/Game/Blueprints/Wind_Bp.Wind_Bp_C|GetDirection _wind) (Variables|/Game/Blueprints/Wind_Bp.Wind_Bp_C|GetSpeed _wind))
          (else
            (CallFunction|SetOceanWaves "1.000000, 0, 0" 1e+01)))))))

(fn SetOceanWaves
  (params (Direction :type Vector) (Speed :type Float%20%28single-precision%29))
  (bind _dynamicmaterial (Variables|Default|GetDynamicMaterial))
  (Rendering|Material|SetVectorParameterValue _dynamicmaterial "Direction" (Math|Conversions|ToLinearColor(Vector) Direction) :!class /Script/Engine.MaterialInstanceDynamic)
  (Rendering|Material|SetScalarParameterValue _dynamicmaterial "Speed" Speed :!class /Script/Engine.MaterialInstanceDynamic))

(fn GetOceanWaves
  (bind _dynamicmaterial (Variables|Default|GetDynamicMaterial))
  (bind _returnvalue (Rendering|Material|GetScalarParameterValue _dynamicmaterial "Amplitde1" :!class /Script/Engine.MaterialInstanceDynamic))
  (bind _returnvalue_2 (Rendering|Material|GetScalarParameterValue _dynamicmaterial "Amplitde2" :!class /Script/Engine.MaterialInstanceDynamic))
  (bind _returnvalue_3 (Rendering|Material|GetScalarParameterValue _dynamicmaterial "Wavelength1" :!class /Script/Engine.MaterialInstanceDynamic))
  (bind _returnvalue_4 (Rendering|Material|GetScalarParameterValue _dynamicmaterial "Wavelength2" :!class /Script/Engine.MaterialInstanceDynamic))
  (bind _returnvalue_5 (Rendering|Material|GetVectorParameterValue _dynamicmaterial "Direction" :!class /Script/Engine.MaterialInstanceDynamic))
  (return _returnvalue _returnvalue_2 _returnvalue_3 _returnvalue_4 (Math|Conversions|ToVector(LinearColor) _returnvalue_5)))