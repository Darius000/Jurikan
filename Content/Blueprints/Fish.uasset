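; Fish actor in a boat game that reacts when the Boat overlaps its sphere.
; Enemy fish damage the boat, while others play a pickup sound; both kinds then add their points to the BoatFishGame game mode's HUD and destroy themselves.
; The construction script randomizes each fish's point value and its color through a dynamic material instance.
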(event OnComponentBeginOverlap(Sphere)
  (params (OverlappedComponent :type Primitive%20Component%20Object%20Reference) (OtherActor :type Actor%20Object%20Reference) (OtherComp :type Primitive%20Component%20Object%20Reference) (OtherBodyIndex :type Integer) (bFromSweep :type Boolean) (SweepResult :type Hit%20Result%20Structure%20%28by%20ref%29))
  (bind _asboat (Utilities|Casting|CastToBoat OtherActor))
  (if (Variables|Default|GetEnemy?)
    (Game|Damage|ApplyDamage _asboat (Variables|Default|GetDamage) 0 self)
    (else
      (Audio|PlaySoundatLocation "/Game/Sound/item_pickup_sound.item_pickup_sound" (Transformation|GetActorLocation))))
  (bind _asboat_fish_game (Utilities|Casting|CastToBoatFishGame (Game|GetGameMode)))
  (Default|AddPoints (Variables|/Game/Blueprints/BoatFishGame.BoatFishGame_C|GetHUD _asboat_fish_game) (Variables|Default|GetPoints))
  (Actor|DestroyActor))

(event EventBeginPlay)

(event Collision|EventActorBeginOverlap
  (params (OtherActor :type Actor%20Object%20Reference)))

(event EventTick
  (params (DeltaSeconds :type Float%20%28single-precision%29)))

(fn ConstructionScript
  (bind _returnvalue (Math|Random|RandomFloatinRange 0.0 1e+01))
  (bind _returnvalue_2 (Rendering|Material|CreateDynamicMaterialInstance (Variables|Character|GetMesh) 0 "/Game/Geometry/Skeletal/skin_texture.skin_texture" :!class /Script/Engine.PrimitiveComponent))
  (Variables|Default|SetFishMat _returnvalue_2)
  (Rendering|Material|SetScalarParameterValue (Variables|Default|GetFishMat) "ColorChange" _returnvalue :!class /Script/Engine.MaterialInstanceDynamic)
  (Variables|Default|SetPoints (Math|Float|Ceil _returnvalue)))