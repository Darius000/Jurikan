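; Player-controlled boat that rides ocean waves, takes damage from fish and can be healed through HealBoat.
; Input turns it by yaw and moves it along its right vector, always in one direction.
; Each tick sets its height from OceanManager wave math, using OceanBp wave parameters and starting sea level.
; Only Fish-caused damage lowers health; a damage event at zero health ends the game, disables input and enables gravity.
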(event EventBeginPlay
  (bind _returnvalue (Transformation|GetActorLocation))
  (bind (_x _y) (Math|Vector|BreakVector _returnvalue))
  ;[1 1 1] Set Offset for boat start
  (bind _output_get (Variables|Default|SetStartLocation (Math|Vector|MakeVector _x _y (.Z (Math|Vector|BreakVector (Transformation|GetActorLocation (Variables|Default|GetOceanBp)))))))
  (Transformation|SetActorLocation _output_get false false))

(event Collision|EventHit
  (params (MyComp :type Primitive%20Component%20Object%20Reference) (Other :type Actor%20Object%20Reference) (OtherComp :type Primitive%20Component%20Object%20Reference) (bSelfMoved :type Boolean) (HitLocation :type Vector :default "0, 0, 0") (HitNormal :type Vector :default "0, 0, 0") (NormalImpulse :type Vector :default "0, 0, 0") (Hit :type Hit%20Result%20Structure%20%28by%20ref%29))
  (Game|Damage|ApplyDamage self 1.0 0 0))

(event EventTick
  (params (DeltaSeconds :type Float%20%28single-precision%29))
  (bind _returnvalue (Transformation|GetActorLocation))
  ;[1 1 1] Ocean Offset on Boat
  (bind (_amp1 _amp2 _wave1 _wav2 _direction) (Default|GetOceanWaves (Variables|Default|GetOceanBp)))
  (bind _returnvalue_2 (Class|OceanManager|GetWaveHeightValue (Variables|Default|GetOceanManager) _wave1 _wav2 _amp1 _amp2 (Transformation|GetActorLocation) (Math|Conversions|ToVector2D(Vector) _direction) (Utilities|Time|GetGameTimeinSeconds)))
  (Transformation|SetActorLocation (Math|Vector|MakeVector (.x _returnvalue) (.y _returnvalue) (+ (.z (Variables|Default|GetStartLocation)) (.Z (Math|Vector|BreakVector _returnvalue_2)))) true false))

(event EventWind
  (params (Direction :type Vector) (Speed :type Float%20%28single-precision%29)))

(event Game|Damage|EventAnyDamage
  (params (Damage :type Float%20%28single-precision%29) (DamageType :type Damage%20Type%20Object%20Reference) (InstigatedBy :type Controller%20Object%20Reference) (DamageCauser :type Actor%20Object%20Reference))
  (bind _boat (Variables|Default|GetBoat))
  ;[1 1 1] Take Damage
  (Utilities|Casting|CastToFish DamageCauser)
  (if (> (Variables|Default|GetHealth) 0.0)
    (Variables|Default|SetHealth (- (Variables|Default|GetHealth) Damage))
    (Audio|PlaySoundatLocation "/Game/Sound/damage_sound.damage_sound" (Transformation|GetActorLocation))
    (Default|CallRecieveDamage)
    (else
      (Variables|Default|SetGameOver true)
      (Audio|PlaySoundatLocation "/Game/Sound/Die_sound.Die_sound" (Transformation|GetActorLocation))
      (Input|DisableInput (Game|GetPlayerController 0))
      (Physics|SetEnableGravity _boat true)
      (Class|PrimitiveComponent|SetConstraintMode _boat "Default"))))

(event Input|AxisEvents|InputAxisMoveForward
  (params (AxisValue :type Float%20%28single-precision%29))
  ;[1 1 1] Move Boat Forward
  (Transformation|SetActorLocation (+ (Transformation|GetActorLocation) (* (Transformation|GetActorRightVector) (* (Math|Float|Absolute(Float) AxisValue) (Variables|Default|GetRate)))) true false))

(event Input|AxisEvents|InputAxisMoveRight
  (params (AxisValue :type Float%20%28single-precision%29))
  ;[1 1 1] Rotate Boat
  (Transformation|SetActorRotation (Math|Rotator|Lerp(Rotator) (Transformation|GetActorRotation) (Math|Rotator|MakeRotator 0.0 0.0 (+ (.Yaw (Math|Rotator|BreakRotator (Transformation|GetActorRotation))) (Variables|Default|GetRotationRate))) AxisValue)))

(fn ConstructionScript
  (|CallParentFunction))

(fn HealBoat
  (params (Recover :type Float%20%28single-precision%29))
  (Variables|Default|SetHealth (+ (Variables|Default|GetHealth) Recover)))